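; Level segment of an endless chain, with scattered scenery and a bridge that opens only while the player's weight is within range.
; Entering it raises the level, scores the active segment by completion speed, rolls the weight range and spawns animals toward that weight, plus random enemies and power-ups.
; Timelines carry player and camera across the bridge.
; Camera overlap makes the game mode create another segment and destroys this one with its spawns.
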(event `self.ReceiveDestroyed`
  ;[1 1 1] Destroy Env
  (`self.RemoveAnimalsFromEnv`)
  (`self.RemovePowerUpsFromEnv`))

(event `self.ReceiveBeginPlay`
  (bind _asbp_top_down_game_mode (`self.GetGameMode`))
  (bind _leftfieldboundmin (`self.LeftFieldBoundMin`))
  (bind _leftfieldboundmax (`self.LeftFieldBoundMax`))
  (bind _rightfieldboundmin (`self.RightFieldBoundMin`))
  (bind _rightfieldboundmax (`self.RightFieldBoundMax`))
  ;[1 1 1] Get Game Mode and Bind Events
  (set `self.GameMode` _asbp_top_down_game_mode)
  (remove `/Game/Blueprints/BP_TopDownGameMode.EventIncreaseGameParameters` _asbp_top_down_game_mode (delegate `IncreaseLevelPointsOnLevel`))
  (`|ExecutionSequence`
    (:`then_0`
      ;[1 1 1] Trees In Left Field
      (`self.GenerateElementsInBounds` _leftfieldboundmin _leftfieldboundmax (`self.NumberOfTrees`) (`self.Trees`) (0.1 0.1 0.1) true)
      ;[1 1 1] Other Meshes In Left Field
      (`self.GenerateElementsInBounds` _leftfieldboundmin _leftfieldboundmax (`self.NumberOfOtherMeshes`) (`self.OtherMeshes`) (1.0 1.0 1.0) true)
      ;[1 1 1] Generate Elements Next To Bridge Left
      (`self.GenerateElementsInBounds` (`self.LeftBridgeBoundMin`) (`self.LeftBridgeBoundMax`) (`self.NumberOfBrdgeMeshes`) (`self.BridgeMeshes`)))
    (:`then_1`
      ;[1 1 1] Trees In Right Field
      (`self.GenerateElementsInBounds` _rightfieldboundmin _rightfieldboundmax (`self.NumberOfTrees`) (`self.Trees`) (0.1 0.1 0.1) true)
      ;[1 1 1] Other Meshes In Right Field
      (`self.GenerateElementsInBounds` _rightfieldboundmin _rightfieldboundmax (`self.NumberOfOtherMeshes`) (`self.OtherMeshes`) (1.0 1.0 1.0) true)
      ;[1 1 1] Generate Elements Next to Bridge Right
      (`self.GenerateElementsInBounds` (`self.RightBridgeBoundMin`) (`self.RightBridgeBoundMax`) (`self.NumberOfBrdgeMeshes`) (`self.BridgeMeshes`)))))

(event `IncreaseLevelPointsOnLevel`
  (bind _asbp_top_down_game_mode (`self.GetGameMode`))
  ;[1 1 1] Event On Level Increase Based On Difficulty
  (`/Engine/EditorBlueprintResources/StandardMacros.IsValid` _asbp_top_down_game_mode
    (:`Is Valid`
      (set `self.PointsLevelCompleted` (`KismetMathLibrary.FTrunc` (* (`self.PointsLevelCompleted`) (`/Game/Blueprints/BP_TopDownGameMode.PointsMultiplier` _asbp_top_down_game_mode)))))))

(event `self.Box.OnComponentBeginOverlap`
  (params (OverlappedComponent :type "PrimitiveComponent Object Reference") (OtherActor :type "Actor Object Reference") (OtherComp :type "PrimitiveComponent Object Reference") (OtherBodyIndex :type Integer) (bFromSweep :type Boolean) (SweepResult :type "HitResult Structure (by ref)"))
  ;[1 1 1] Overalpping camera destroy env and create a new one
  (cast `/Game/Blueprints/Environment/BP_Camera` OtherActor)
  (`/Game/Blueprints/BP_TopDownGameMode.CreateNewEnv` (`self.GetGameMode`))
  (`self.K2_DestroyActor`))

(event `self.ReceiveTick`
  (params (DeltaSeconds :type "Float (single-precision)"))
  ;[1 1 1] Update Door
  (if (`KismetMathLibrary.InRange_FloatFloat` (`self.PlayerCurrentWeight`) (`self.MinBridgeWeight`) (`self.MaxBridgeWeight`))
    (`self.AllowEntrance`)
    (else
      (`self.ForbidEntrance`))))

(event `self.ChangeEnv.OnComponentBeginOverlap`
  (params (OverlappedComponent :type "PrimitiveComponent Object Reference") (OtherActor :type "Actor Object Reference") (OtherComp :type "PrimitiveComponent Object Reference") (OtherBodyIndex :type Integer) (bFromSweep :type Boolean) (SweepResult :type "HitResult Structure (by ref)"))
  (bind _asbp_top_down_game_mode (`self.GetGameMode`))
  ;[1 1 1] Set Current Environment
  (`/Engine/EditorBlueprintResources/StandardMacros.IsValid` OtherActor
    (:`Is Valid`
      (cast `/Game/Blueprints/Characters/BP_MainCharacter` OtherActor)
      (if (not (`self.IsLevelIncreased`))
        (set `self.IsLevelIncreased` true)
        (`/Game/Blueprints/BP_TopDownGameMode.IncreaseLevel` _asbp_top_down_game_mode)
        (`self.AddLevelPoints` (`/Game/Blueprints/BP_TopDownGameMode.ActiveEnv` _asbp_top_down_game_mode))
        (`/Game/Blueprints/BP_TopDownGameMode.SetActiveEnvironment` _asbp_top_down_game_mode self)
        (`self.CalculateNewMinAndMaxWeight`)
        ;[1 1 1] Spawn Animals in Env
        (`self.InitializeSpawnPoints`)
        (`self.Initialize Env Spawn Points`)
        (`self.Spawn Env In the Path`)
        (`self.SpawnAnimals`)
        (`self.SetInitialTime`)))))

(event `self.ChangeEnv1.OnComponentBeginOverlap`
  (params (OverlappedComponent :type "PrimitiveComponent Object Reference") (OtherActor :type "Actor Object Reference") (OtherComp :type "PrimitiveComponent Object Reference") (OtherBodyIndex :type Integer) (bFromSweep :type Boolean) (SweepResult :type "HitResult Structure (by ref)"))
  ;[1 1 1] Close Bridge to go back
  (`/Engine/EditorBlueprintResources/StandardMacros.IsValid` OtherActor
    (:`Is Valid`
      (cast `/Game/Blueprints/Characters/BP_MainCharacter` OtherActor)
      (`PrimitiveComponent.SetCollisionResponseToChannel` (`self.ChangeEnv`) "ECC_Pawn" "ECR_Block"))))

(event `self.PassBridgeBox.OnComponentBeginOverlap`
  (params (OverlappedComponent :type "PrimitiveComponent Object Reference") (OtherActor :type "Actor Object Reference") (OtherComp :type "PrimitiveComponent Object Reference") (OtherBodyIndex :type Integer) (bFromSweep :type Boolean) (SweepResult :type "HitResult Structure (by ref)"))
  (bind _returnvalue_x (`KismetMathLibrary.BreakVector` (`SceneComponent.K2_GetComponentLocation` (`self.PassBridgeBox`))))
  (bind _returnvalue_x_2 (`KismetMathLibrary.BreakVector` (`SceneComponent.K2_GetComponentLocation` (`self.AttachPoint`))))
  ;[1 1 1] Player Begin Cross Bridge
  (`/Engine/EditorBlueprintResources/StandardMacros.IsValid` OtherActor
    (:`Is Valid`
      (bind _asbp_main_character (cast `/Game/Blueprints/Characters/BP_MainCharacter` OtherActor))
      (`/Engine/EditorBlueprintResources/StandardMacros.IsValid` _asbp_main_character
        (:`Is Valid`
          (`/Game/Blueprints/BP_TopDownGameMode.Play Sound Effect` (`self.GetGameMode`) "/Game/Audio/SFX/transport.transport")
          (`|ExecutionSequence`
            (:`then_0`
              ;[1 1 1] Transport Player
              (bind (_direction _alpha) (`Timeline|MoveCharacterToEndOfBridge` :!via `PlayFromStart` :!label _label)
                (:`Update`
                  (`/Engine/EditorBlueprintResources/StandardMacros.IsValid` _asbp_main_character
                    (:`Is Valid`
                      (bind _capsulecomponent (`Character.CapsuleComponent` _asbp_main_character))
                      (`/Engine/EditorBlueprintResources/StandardMacros.IsValid` _capsulecomponent
                        (:`Is Valid`
                          (bind _returnvalue (`SceneComponent.K2_GetComponentToWorld` _capsulecomponent))
                          (`SceneComponent.K2_SetWorldTransform` _capsulecomponent (`KismetMathLibrary.MakeTransform` (`KismetMathLibrary.VLerp` (`KismetMathLibrary.MakeVector` (.x (.location _returnvalue)) (.y (.location _returnvalue)) (.z (.location _returnvalue))) (`KismetMathLibrary.MakeVector` _returnvalue_x_2 (.y (.location _returnvalue)) (.z (.location _returnvalue))) _alpha) (.rotation _returnvalue) (.scale _returnvalue)) false false))))))))
            (:`then_1`
              ;[1 1 1] Transport Camera
              (bind _returnvalue_2 (`GameplayStatics.GetActorOfClass` "/Game/Blueprints/Environment/BP_Camera.BP_Camera_C"))
              (`/Engine/EditorBlueprintResources/StandardMacros.IsValid` _returnvalue_2
                (:`Is Valid`
                  (bind (_direction_2 _alpha_2) (`Timeline|MoveCameraToBridge` :!via `PlayFromStart` :!label _label_2)
                    (:`Update`
                      (bind _camera (`/Game/Blueprints/Environment/BP_Camera.Camera` _returnvalue_2))
                      (`/Engine/EditorBlueprintResources/StandardMacros.IsValid` _camera
                        (:`Is Valid`
                          (bind _returnvalue_3 (`SceneComponent.K2_GetComponentToWorld` _camera))
                          (`SceneComponent.K2_SetWorldTransform` _camera (`KismetMathLibrary.MakeTransform` (`KismetMathLibrary.VLerp` (`KismetMathLibrary.MakeVector` (.x (.location _returnvalue_3)) (.y (.location _returnvalue_3)) (.z (.location _returnvalue_3))) (`KismetMathLibrary.MakeVector` (- _returnvalue_x 0.0) (.y (.location _returnvalue_3)) (.z (.location _returnvalue_3))) _alpha_2) (.rotation _returnvalue_3) (.scale _returnvalue_3)) false false))))))))))))))

(event `self.PassBridgeBox1.OnComponentBeginOverlap`
  (params (OverlappedComponent :type "PrimitiveComponent Object Reference") (OtherActor :type "Actor Object Reference") (OtherComp :type "PrimitiveComponent Object Reference") (OtherBodyIndex :type Integer) (bFromSweep :type Boolean) (SweepResult :type "HitResult Structure (by ref)"))
  ;[1 1 1] Player End Cross Bridge
  (`/Engine/EditorBlueprintResources/StandardMacros.IsValid` OtherActor
    (:`Is Valid`
      (cast `/Game/Blueprints/Characters/BP_MainCharacter` OtherActor)
      (`|ExecutionSequence`
        (:`then_0`
          (goto _label :!via `Stop`))
        (:`then_1`
          (goto _label_2 :!via `Stop`))))))

(fn `AddLevelPoints`
  (bind _asbp_top_down_game_mode (`self.GetGameMode`))
  (bind _timeinseconds (`self.GetTimeInLevel`))
  (if (< _timeinseconds 5.0)
    (`/Game/Blueprints/BP_TopDownGameMode.AddPointsToCurrentScore` _asbp_top_down_game_mode (* (`self.PointsLevelCompleted`) 3))
    (elif (< _timeinseconds 8.0)
      (`/Game/Blueprints/BP_TopDownGameMode.AddPointsToCurrentScore` _asbp_top_down_game_mode (* (`self.PointsLevelCompleted`) 2))
      (else
        (`/Game/Blueprints/BP_TopDownGameMode.AddPointsToCurrentScore` _asbp_top_down_game_mode (`self.PointsLevelCompleted`))))))

(fn `AllowEntrance`
  (`ActorComponent.Deactivate` (`self.ParticleSystem1`))
  (`ActorComponent.Deactivate` (`self.ParticleSystem`))
  (`PrimitiveComponent.SetCollisionEnabled` (`self.StopWall`) "NoCollision")
  (`LightComponent.SetLightColor` (`self.ColorBridgeEnableLight`) (`KismetMathLibrary.LinearColor_Green`) true))

(fn `CalculateNewMinAndMaxWeight`
  (bind _weight (`self.PlayerCurrentWeight`))
  (bind _returnvalue (/ (`/Game/Blueprints/BP_TopDownGameMode.MaxBridgeWeight` (`self.GetGameMode`)) 2.0))
  (if (> _weight _returnvalue)
    (bind _output_get (set `self.MinBridgeWeight` (`KismetMathLibrary.Conv_IntToDouble` (`KismetMathLibrary.Round` (`KismetMathLibrary.RandomFloatInRange` 0.0 _returnvalue)))))
    (set `self.MaxBridgeWeight` (`KismetMathLibrary.Conv_IntToDouble` (`KismetMathLibrary.Round` (`KismetMathLibrary.RandomFloatInRange` (+ _output_get 50.0) (+ _output_get (`self.BridgeWeightMaxGap`))))))
    (else
      (bind _output_get_2 (set `self.MinBridgeWeight` (`KismetMathLibrary.Conv_IntToDouble` (`KismetMathLibrary.Round` (`KismetMathLibrary.RandomFloatInRange` _weight (+ _weight 100.0))))))
      (set `self.MaxBridgeWeight` (`KismetMathLibrary.Conv_IntToDouble` (`KismetMathLibrary.Round` (`KismetMathLibrary.RandomFloatInRange` (+ _output_get_2 50.0) (+ _output_get_2 (`self.BridgeWeightMaxGap`)))))))))

(fn `ForbidEntrance`
  (`ActorComponent.Activate` (`self.ParticleSystem1`) false)
  (`ActorComponent.Activate` (`self.ParticleSystem`) false)
  (`PrimitiveComponent.SetCollisionEnabled` (`self.StopWall`) "QueryAndPhysics")
  (`LightComponent.SetLightColor` (`self.ColorBridgeEnableLight`) (`KismetMathLibrary.LinearColor_Red`) true))

(fn `GenerateElementsInBounds`
  (params (MinBound :type "Vector Structure") (MaxBound :type "Vector Structure") (NumElements :type Integer) (Components :type "Array of StaticMesh Object Reference") (Scale :type "Vector Structure" :default (1.0 1.0 1.0)) (RandomizeNumber :type Boolean))
  (bind _returnvalue (`KismetMathLibrary.Conv_VectorToTransform` (`KismetMathLibrary.RandomPointInBoundingBox_Box` (make `Box` MinBound MaxBound))))
  (if RandomizeNumber
    (for _ (range 1 (+ (`KismetMathLibrary.FFloor` (* NumElements (`KismetMathLibrary.RandomFloatInRange` 0.5 1.0))) 1))
      (bind _returnvalue_2 (`AddComponent|NODE_AddInstancedStaticMeshComponent-3` :!label _label))
      (`StaticMeshComponent.SetStaticMesh` _returnvalue_2 (`|GetArrayItem` Components (`KismetMathLibrary.RandomInteger` (`KismetArrayLibrary.Array_Length` Components))))
      (`InstancedStaticMeshComponent.AddInstance` _returnvalue_2 (`KismetMathLibrary.MakeTransform` (.location _returnvalue) (`KismetMathLibrary.MakeRotator` (.roll (.rotation _returnvalue)) (.pitch (.rotation _returnvalue)) (* (.yaw (.rotation _returnvalue)) (`KismetMathLibrary.RandomFloatInRange` 90.0 180.0))) Scale) false))
    (else
      (for _ (range 1 (+ NumElements 1))
        (goto _label)))))

(fn `GetAttachPoint`
  (returns (ReturnValue :type "Transform Structure"))
  (return (`SceneComponent.K2_GetComponentToWorld` (`self.AttachPoint`))))

(fn `GetGameMode`
  (returns (`AsBP Top Down Game Mode` :type "/Game/Blueprints/BP_TopDownGameMode Object Reference"))
  (bind _asbp_top_down_game_mode (cast `/Game/Blueprints/BP_TopDownGameMode` (`GameplayStatics.GetGameMode`)))
  (return _asbp_top_down_game_mode))

(fn `GetTimeInLevel`
  (returns (TimeInSeconds :type "Float (double-precision)"))
  (return (- (`KismetSystemLibrary.GetGameTimeInSeconds`) (`self.SecondsAtLevelBegin`))))

(fn `Initialize Env Spawn Points`
  (for _array_element (`self.GetComponentsByTag` "/Script/Engine.ArrowComponent" "EnvSpawnPoint")
    (`KismetArrayLibrary.Array_Add` (`self.EnvSpawnPoints`) _array_element)))

(fn `InitializeSpawnPoints`
  (for _array_element (`self.GetComponentsByTag` "/Script/Engine.ArrowComponent" "SpawnPoint")
    (`KismetArrayLibrary.Array_Add` (`self.SpawnPoints`) _array_element)))

(fn `Pick Random Unused Spawn Point And Mark`
  (returns (PickedItem :type "ArrowComponent Object Reference"))
  (bind _spawnpoints (`self.SpawnPoints`))
  (bind _usedspawnpoints (`self.UsedSpawnPoints`))
  (bind _returnvalue (`KismetArrayLibrary.Array_Length` _spawnpoints))
  (bind _outitem (`KismetArrayLibrary.Array_Random` _spawnpoints))
  (for _index (range 1 (+ _returnvalue 1))
    (`/Engine/EditorBlueprintResources/StandardMacros.IsValid` _outitem
      (:`Is Valid`
        (if (not (`KismetArrayLibrary.Array_Contains` _usedspawnpoints))
          (`KismetArrayLibrary.Array_Add` _usedspawnpoints _outitem)
          (break)))))
  (if (>= _index _returnvalue)
    (return null)
    (else
      (return _outitem))))

(fn `PlayerCurrentWeight`
  (returns (Weight :type "Float (double-precision)"))
  (return (`/Game/Blueprints/BP_TopDownGameMode.CurrentPlayerWeight` (`self.GameMode`))))

(fn `RemoveAnimalsFromEnv`
  (for _array_element (`self.SpawnedAnimals`)
    (`/Engine/EditorBlueprintResources/StandardMacros.IsValid` _array_element
      (:`Is Valid`
        (`self.K2_DestroyActor` _array_element)))))

(fn `RemovePowerUpsFromEnv`
  (for _array_element (`self.SpawnedPowerUps`)
    (`/Engine/EditorBlueprintResources/StandardMacros.IsValid` _array_element
      (:`Is Valid`
        (`self.K2_DestroyActor` _array_element)))))

(fn `SetInitialTime`
  (set `self.SecondsAtLevelBegin` (`KismetSystemLibrary.GetGameTimeInSeconds`)))

(fn `Spawn Env In the Path`
  (for _array_element (`self.EnvSpawnPoints`)
    (bind _returnvalue (`AddComponent|NODE_AddInstancedStaticMeshComponent-4`))
    (`StaticMeshComponent.SetStaticMesh` _returnvalue (`KismetArrayLibrary.Array_Random` (`self.MeshesForPath`)))
    (`InstancedStaticMeshComponent.AddInstance` _returnvalue (`SceneComponent.K2_GetComponentToWorld` _array_element) true)))

(fn `Spawn Random Number at Random Locations`
  (bind _spawnedanimals (`self.SpawnedAnimals`))
  (for _ (range 1 (+ (`KismetMathLibrary.RandomIntegerInRange` 1 (`KismetArrayLibrary.Array_Length` (`self.SpawnPoints`))) 1))
    (bind _pickeditem (`self.Pick Random Unused Spawn Point And Mark`))
    (`/Engine/EditorBlueprintResources/StandardMacros.IsValid` _pickeditem
      (:`Is Valid`
        (if (> (`KismetMathLibrary.RandomIntegerInRange` 0 100) (`self.ProbabilityEnemySpawn`))
          (bind _spawnedanimal (`self.SpawnAnimalAtLocation` (`KismetArrayLibrary.Array_Random` (`self.SpawnableAnimals`)) _pickeditem))
          (`KismetArrayLibrary.Array_Add` _spawnedanimals _spawnedanimal)
          (elif (> (`KismetMathLibrary.RandomIntegerInRange` 0 100) 50)
            (bind _spawnedanimal_2 (`self.SpawnAnimalAtLocation` (`KismetArrayLibrary.Array_Random` (`self.SpawnableEnemies`)) _pickeditem))
            (`KismetArrayLibrary.Array_Add` _spawnedanimals _spawnedanimal_2)
            (else
              (bind _spawnedpowerup (`self.SpawnPowerUpAtLocation` (`KismetArrayLibrary.Array_Random` (`self.SpawnablePowerUps`)) _pickeditem))
              (`KismetArrayLibrary.Array_Add` (`self.SpawnedPowerUps`) _spawnedpowerup))))))))

(fn `SpawnAnimalAtLocation`
  (params (AnimalClass :type "/Game/Blueprints/Animals/BP_Animal Class Reference") (SceneComponent :type "ArrowComponent Object Reference"))
  (returns (SpawnedAnimal :type "/Game/Blueprints/Animals/BP_Animal Object Reference"))
  (bind _returnvalue (`SceneComponent.K2_GetComponentToWorld` SceneComponent))
  (bind _returnvalue_2 (`|SpawnActorFromClass` AnimalClass (`KismetMathLibrary.MakeTransform` (`KismetMathLibrary.MakeVector` (.x (.location _returnvalue)) (+ (.y (.location _returnvalue)) (`KismetMathLibrary.RandomFloatInRange` -400.0 400.0)) (.z (.location _returnvalue))) (`KismetMathLibrary.MakeRotator` (.roll (.rotation _returnvalue)) (.pitch (.rotation _returnvalue)) (`KismetMathLibrary.RandomFloatInRange` 0.0 360.0)) (.scale _returnvalue)) "Undefined" "MultiplyWithRoot" null null))
  (`/Engine/EditorBlueprintResources/StandardMacros.IsValid` _returnvalue_2
    (:`Is Valid`
      (bind (_returnvalue_x _returnvalue_y) (`KismetMathLibrary.BreakVector` (`self.K2_GetActorLocation` _returnvalue_2)))
      (`self.K2_SetActorLocation` _returnvalue_2 (`KismetMathLibrary.MakeVector` _returnvalue_x _returnvalue_y 10.0) true false)
      (return _returnvalue_2))))

(fn `SpawnAnimals`
  (bind _weight (`self.PlayerCurrentWeight`))
  (if (> _weight (`self.MaxBridgeWeight`))
    (`self.Spawn Random Number at Random Locations`)
    (else
      (set `self.EnvCalculatedWeight` _weight)
      (`self.SpawnAnimalsToReachEnvWeight`))))

(fn `SpawnAnimalsToReachEnvWeight`
  (for _ (range 1 (+ (`KismetArrayLibrary.Array_Length` (`self.SpawnPoints`)) 1))
    (bind _pickeditem (`self.Pick Random Unused Spawn Point And Mark`))
    (`/Engine/EditorBlueprintResources/StandardMacros.IsValid` _pickeditem
      (:`Is Valid`
        (bind _spawnedanimal (`self.SpawnAnimalAtLocation` (`KismetArrayLibrary.Array_Random` (`self.SpawnableAnimals`)) _pickeditem))
        (`/Engine/EditorBlueprintResources/StandardMacros.IsValid` _spawnedanimal
          (:`Is Valid`
            (`KismetArrayLibrary.Array_Add` (`self.SpawnedAnimals`) _spawnedanimal)
            (bind _output_get (set `self.EnvCalculatedWeight` (+ (`/Game/Blueprints/Animals/BP_Animal.Weight` _spawnedanimal) (`self.EnvCalculatedWeight`))))
            (if (< (`self.MinBridgeWeight`) _output_get)
              (break)))))))
  (`self.Spawn Random Number at Random Locations`))

(fn `SpawnPowerUpAtLocation`
  (params (PowerUpClass :type "/Game/Blueprints/PowerUps/BP_PowerUp Class Reference") (SceneComponent :type "ArrowComponent Object Reference"))
  (returns (SpawnedPowerUp :type "/Game/Blueprints/PowerUps/BP_PowerUp Object Reference"))
  (bind _returnvalue (`SceneComponent.K2_GetComponentToWorld` SceneComponent))
  (bind _returnvalue_2 (`|SpawnActorFromClass` PowerUpClass (`KismetMathLibrary.MakeTransform` (`KismetMathLibrary.MakeVector` (.x (.location _returnvalue)) (+ (.y (.location _returnvalue)) (`KismetMathLibrary.RandomFloatInRange` -400.0 400.0)) (.z (.location _returnvalue))) (.rotation _returnvalue) (.scale _returnvalue)) "Undefined" "MultiplyWithRoot" null null))
  (return _returnvalue_2))

(fn `UserConstructionScript`)