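; BP_Camera is a camera Blueprint that scrolls its camera continuously along world X and speeds up as game difficulty increases.
; Tick offsets the camera by CameraSpeed scaled by delta time, keeping the other axes, rotation and scale unchanged.
; On BeginPlay it binds to BP_TopDownGameMode's IncreaseGameParameters event, which multiplies CameraSpeed by the game mode's SpeedMultiplier and truncates the result to an integer.
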(event `self.ReceiveBeginPlay`
  ;[1 1 1] Bind Speed to Difficulty Level
  (bind _asbp_top_down_game_mode (cast `/Game/Blueprints/BP_TopDownGameMode` (`GameplayStatics.GetGameMode`)))
  (`/Engine/EditorBlueprintResources/StandardMacros.IsValid` _asbp_top_down_game_mode
    (:`Is Valid`
      (add `/Game/Blueprints/BP_TopDownGameMode.EventIncreaseGameParameters` _asbp_top_down_game_mode (delegate `IncreaseCameraSpeed`)))))

(event `IncreaseCameraSpeed`
  ;[1 1 1] Bind Speed to Difficulty Level
  (`/Engine/EditorBlueprintResources/StandardMacros.IsValid` (stale `self.ReceiveBeginPlay` _asbp_top_down_game_mode)
    (:`Is Valid`
      (set `self.CameraSpeed` (`KismetMathLibrary.FTrunc` (* (`self.CameraSpeed`) (`/Game/Blueprints/BP_TopDownGameMode.SpeedMultiplier` (stale `self.ReceiveBeginPlay` _asbp_top_down_game_mode))))))))

(event `self.ReceiveTick`
  (params (DeltaSeconds :type "Float (single-precision)"))
  (bind _returnvalue (`SceneComponent.K2_GetComponentToWorld` (`self.Camera`)))
  ;[1 1 1] Camera movement
  (`SceneComponent.K2_SetWorldTransform` (`self.Camera`) (`KismetMathLibrary.MakeTransform` (`KismetMathLibrary.MakeVector` (+ (.x (.location _returnvalue)) (* DeltaSeconds (`self.CameraSpeed`))) (.y (.location _returnvalue)) (.z (.location _returnvalue))) (.rotation _returnvalue) (.scale _returnvalue)) false false))

(fn `UserConstructionScript`)