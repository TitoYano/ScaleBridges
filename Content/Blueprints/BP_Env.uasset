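; BP_Env is an environment segment that decorates itself and is replaced as the camera moves through it.
; On BeginPlay it scatters random trees, other meshes and bridge-side props within left and right bounds, randomizing field counts and creating one instanced mesh component per element.
; When BP_Camera overlaps its Box, it has BP_TopDownGameMode create a new environment and destroys itself.
; GetAttachPoint exposes the world transform of its attach point.
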(event `self.ReceiveBeginPlay`
  (bind _leftfieldboundmin (`self.LeftFieldBoundMin`))
  (bind _leftfieldboundmax (`self.LeftFieldBoundMax`))
  (bind _rightfieldboundmin (`self.RightFieldBoundMin`))
  (bind _rightfieldboundmax (`self.RightFieldBoundMax`))
  (`|ExecutionSequence`
    (:`then_0`
      ;[1 1 1] Trees In Left Field
      (`self.GenerateElementsInBounds` _leftfieldboundmin _leftfieldboundmax (`self.NumberOfTrees`) (`self.Trees`) (0.1 0.1 0.1) true)
      ;[1 1 1] Other Meshes In Left Field
      (`self.GenerateElementsInBounds` _leftfieldboundmin _leftfieldboundmax (`self.NumberOfOtherMeshes`) (`self.OtherMeshes`) (1.0 1.0 1.0) true)
      ;[1 1 1] Generate Elements Next To Bridge Left
      (`self.GenerateElementsInBounds` (`self.LeftBridgeBoundMin`) (`self.LeftBridgeBoundMax`) (`self.NumberOfBrdgeMeshes`) (`self.BridgeMeshes`)))
    (:`then_1`
      ;[1 1 1] Trees In Right Field
      (`self.GenerateElementsInBounds` _rightfieldboundmin _rightfieldboundmax (`self.NumberOfTrees`) (`self.Trees`) (0.1 0.1 0.1) true)
      ;[1 1 1] Other Meshes In Right Field
      (`self.GenerateElementsInBounds` _rightfieldboundmin _rightfieldboundmax (`self.NumberOfOtherMeshes`) (`self.OtherMeshes`) (1.0 1.0 1.0) true)
      ;[1 1 1] Generate Elements Next to Bridge Right
      (`self.GenerateElementsInBounds` (`self.RightBridgeBoundMin`) (`self.RightBridgeBoundMax`) (`self.NumberOfBrdgeMeshes`) (`self.BridgeMeshes`)))))

(event `self.Box.OnComponentBeginOverlap`
  (params (OverlappedComponent :type "PrimitiveComponent Object Reference") (OtherActor :type "Actor Object Reference") (OtherComp :type "PrimitiveComponent Object Reference") (OtherBodyIndex :type Integer) (bFromSweep :type Boolean) (SweepResult :type "HitResult Structure (by ref)"))
  ;[1 1 1] Overalpping camera destroy env and create a new one
  (cast `/Game/Blueprints/BP_Camera` OtherActor)
  (bind _asbp_top_down_game_mode (cast `/Game/Blueprints/BP_TopDownGameMode` (`GameplayStatics.GetGameMode`)))
  (`/Game/Blueprints/BP_TopDownGameMode.CreateNewEnv` _asbp_top_down_game_mode)
  (`self.K2_DestroyActor`))

(fn `GenerateElementsInBounds`
  (params (MinBound :type "Vector Structure") (MaxBound :type "Vector Structure") (NumElements :type Integer) (Components :type "Array of StaticMesh Object Reference") (Scale :type "Vector Structure" :default (1.0 1.0 1.0)) (RandomizeNumber :type Boolean))
  (bind _returnvalue (`KismetMathLibrary.Conv_VectorToTransform` (`KismetMathLibrary.RandomPointInBoundingBox_Box` (make `Box` MinBound MaxBound))))
  (if RandomizeNumber
    (for _ (range 1 (+ (`KismetMathLibrary.FFloor` (* NumElements (`KismetMathLibrary.RandomFloatInRange` 0.5 1.0))) 1))
      (bind _returnvalue_2 (`AddComponent|NODE_AddInstancedStaticMeshComponent-3` :!label _label))
      (`StaticMeshComponent.SetStaticMesh` _returnvalue_2 (`|GetArrayItem` Components (`KismetMathLibrary.RandomInteger` (`KismetArrayLibrary.Array_Length` Components))))
      (`InstancedStaticMeshComponent.AddInstance` _returnvalue_2 (`KismetMathLibrary.MakeTransform` (.location _returnvalue) (`KismetMathLibrary.MakeRotator` (.roll (.rotation _returnvalue)) (.pitch (.rotation _returnvalue)) (* (.yaw (.rotation _returnvalue)) (`KismetMathLibrary.RandomFloatInRange` 90.0 180.0))) Scale) false))
    (else
      (for _ (range 1 (+ NumElements 1))
        (goto _label)))))

(fn `GetAttachPoint`
  (returns (ReturnValue :type "Transform Structure"))
  (return (`SceneComponent.K2_GetComponentToWorld` (`self.AttachPoint`))))

(fn `UserConstructionScript`)