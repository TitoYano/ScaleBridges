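; Backpack Blueprint that stores collected animals under a weight limit.
; AddNewAnimal rejects any animal that would push the total past MaxWeight, otherwise appends it and increases CurrentWeight.
; RemoveFirstFound removes the first entry of matching Type, subtracting the passed animal's weight rather than the stored entry's.
; Both return a success flag, and SetCurrentWeight clamps every change between MinWeight and MaxWeight.
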(fn `AddNewAnimal`
  (params (NewAnimal :type "/Game/Blueprints/Animals/BP_Animal Object Reference"))
  (returns (Success :type Boolean))
  (bind _weigth (`/Game/Blueprints/Animals/BP_Animal.Weigth` NewAnimal))
  (bind _overloaded (`self.Will Exceed Max` _weigth))
  (if _overloaded
    (return false)
    (else
      (`KismetArrayLibrary.Array_Add` (`self.AnimalsInBag`) NewAnimal)
      (`self.SetCurrentWeight` (+ (`self.CurrentWeight`) _weigth))
      (return true))))

(fn `Remove First Found`
  (params (Animal :type "/Game/Blueprints/Animals/BP_Animal Object Reference"))
  (returns (Success :type Boolean))
  (bind _animalsinbag (`self.AnimalsInBag`))
  (for (_array_element _array_index) _animalsinbag
    (if (== (`/Game/Blueprints/Animals/BP_Animal.Type` _array_element) (`/Game/Blueprints/Animals/BP_Animal.Type` Animal))
      (`self.SetCurrentWeight` (- (`self.CurrentWeight`) (`/Game/Blueprints/Animals/BP_Animal.Weigth` Animal)))
      (break)))
  (if (>= _array_index (`KismetArrayLibrary.Array_Length` _animalsinbag))
    (return false)
    (else
      (`KismetArrayLibrary.Array_Remove` _animalsinbag _array_index)
      (return true))))

(fn `SetCurrentWeight`
  (params (NewWeight :type "Float (double-precision)"))
  (set `self.CurrentWeight` (`KismetMathLibrary.FClamp` NewWeight (`self.MinWeight`) (`self.MaxWeight`))))

(fn `Will Exceed Max`
  (params (Weight :type "Float (double-precision)"))
  (returns (Overloaded :type Boolean))
  (if (> (+ (`self.CurrentWeight`) Weight) (`self.MaxWeight`))
    (return true)
    (else
      (return false))))